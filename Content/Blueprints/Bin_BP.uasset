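; Sorting bin Blueprint that judges whether an actor entering its box trigger is one of its correct objects.
; On overlap it checks the actor against the CorrectObject collection, prints the result and adds a correct or wrong feedback widget to the viewport.
; After a short delay it calls RemoveAllWidgets, which clears every widget in the viewport rather than only the one it created.
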(event `self.Box.OnComponentBeginOverlap`
  (params (OverlappedComponent :type "PrimitiveComponent Object Reference") (OtherActor :type "Actor Object Reference") (OtherComp :type "PrimitiveComponent Object Reference") (OtherBodyIndex :type Integer) (bFromSweep :type Boolean) (SweepResult :type "HitResult Structure (by ref)"))
  (if (`KismetArrayLibrary.Array_Contains` (`self.CorrectObject`) OtherActor)
    (`KismetSystemLibrary.PrintString` "Correct" true true (struct :`G` 1.0 :`B` 0.079329 :`A` 1.0) 10.0)
    (bind _returnvalue (`|CreateWidget` "/Game/Blueprints/CorrectWidget.CorrectWidget_C"))
    (`UserWidget.AddToViewport` _returnvalue 0)
    (else
      (`KismetSystemLibrary.PrintString` "Incorrect" true true (struct :`R` 1.0 :`G` 0.032923 :`B` 0.024965 :`A` 1.0))
      (bind _returnvalue_2 (`|CreateWidget` "/Game/Blueprints/WrongWidget.WrongWidget_C"))
      (`UserWidget.AddToViewport` _returnvalue_2 0)))
  (`KismetSystemLibrary.Delay` 5.0)
  (`WidgetLayoutLibrary.RemoveAllWidgets`))

(fn `UserConstructionScript`)