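; Anti-gravity object actor that rises vertically from its starting location, then spins its cube in place.
; BeginPlay sets a target point raised by an Offset on Z.
; Tick lerps the root toward it using global game time over Duration, rather than the accumulated CurrentTime.
; Once the root is above the target height, Tick instead applies a fixed, frame-rate-dependent local rotation to the Cube.
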(event `self.ReceiveBeginPlay`
  (bind _output_get (set `self.CurrentLocation` (`SceneComponent.K2_GetComponentLocation` (`self.DefaultSceneRoot`))))
  (bind _output_get_2 (set `self.TargetZ` (+ (.z _output_get) (`self.Offset`))))
  (set `self.TargetPosition` (`KismetMathLibrary.MakeVector` (.x _output_get) (.y _output_get) _output_get_2))
  (set `self.Distance` (`KismetMathLibrary.Vector_Distance` (`self.CurrentLocation`) (`self.TargetPosition`))))

(event `self.ReceiveTick`
  (params (DeltaSeconds :type "Float (single-precision)"))
  (set `self.CurrentTime` (+ DeltaSeconds (`self.CurrentTime`)))
  (if (<= (.z (`SceneComponent.K2_GetComponentLocation` (`self.DefaultSceneRoot`))) (`self.TargetZ`))
    (`SceneComponent.K2_SetWorldTransform` (`self.DefaultSceneRoot`) (`KismetMathLibrary.MakeTransform` (`KismetMathLibrary.VLerp` (`self.CurrentLocation`) (`self.TargetPosition`) (/ (`KismetSystemLibrary.GetGameTimeInSeconds`) (`self.Duration`))) (`SceneComponent.K2_GetComponentRotation` (`self.DefaultSceneRoot`)) (`SceneComponent.K2_GetComponentScale` (`self.DefaultSceneRoot`))) false false)
    (else
      (`SceneComponent.K2_AddLocalRotation` (`self.Cube`) (struct :`Pitch` 2.0 :`Yaw` -2.0 :`Roll` 2.0) false false))))

(fn `UserConstructionScript`)